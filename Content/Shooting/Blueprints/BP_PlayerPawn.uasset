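; Player pawn for a shooting game that, as wired, only speeds up the background through two test keys.
; BeginPlay creates a dynamic material instance on BP_Background's mesh; key 1 scales up its SpeedPer parameter.
; Key 2 scales up Speed in the MPCBackground parameter collection instead.
; Enhanced Input setup, movement, sound, effect spawn and destroy nodes are disconnected and never run.
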(event EventBeginPlay
  (bind _returnvalue (Actor|GetActorOfClass "/Game/Shooting/Blueprints/BP_Background.BP_Background_C"))
  (bind _returnvalue_2 (Rendering|Material|CreateDynamicMaterialInstance (Variables|/Script/Engine.StaticMeshActor|GetStaticMeshComponent _returnvalue) 0 (Rendering|Material|GetMaterial (Variables|/Script/Engine.StaticMeshActor|GetStaticMeshComponent _returnvalue) 0) "None" :!class /Script/Engine.PrimitiveComponent))
  (Variables|Default|SetDynamicMat _returnvalue_2))

(event Collision|EventActorBeginOverlap
  (params (OtherActor :type Actor%20Object%20Reference)))

(event EventTick
  (params (DeltaSeconds :type Float%20%28single-precision%29)))

(event Input|KeyboardEvents|1
  (params (Key :type Key%20Structure :default "None"))
  (bind _dynamicmat (Variables|Default|GetDynamicMat))
  (:Pressed
    (bind _returnvalue (Rendering|Material|GetScalarParameterValue _dynamicmat "SpeedPer" :!class /Script/Engine.MaterialInstanceDynamic))
    (Rendering|Material|SetScalarParameterValue _dynamicmat "SpeedPer" (* _returnvalue 1.1) :!class /Script/Engine.MaterialInstanceDynamic)))

(event Input|KeyboardEvents|2
  (params (Key :type Key%20Structure :default "None"))
  (bind _returnvalue (Utilities|Name|MakeLiteralName "Speed"))
  (bind _mpc_background (Variables|Default|GetMPC_Background))
  (:Pressed
    (bind _returnvalue_2 (Rendering|Material|GetScalarParameterValue _mpc_background _returnvalue :!class /Script/Engine.KismetMaterialLibrary))
    (Rendering|Material|SetScalarParameterValue _mpc_background _returnvalue (* _returnvalue_2 1.1) :!class /Script/Engine.KismetMaterialLibrary)))

(fn ConstructionScript)